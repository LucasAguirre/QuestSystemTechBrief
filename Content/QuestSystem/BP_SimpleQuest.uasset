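; Simple quest object that tracks one quest's state from Blocked through Available and InProgress to Completed.
; Blocked quests become Available when their conditions pass an all-or-any rule, or when none exist.
; In progress, it evaluates unfinished objectives and binds their completion events to trigger re-evaluation until all are done.
; Completion unbinds objective events, plays a HUD_Shooter banner and notifies the player controller.
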(event `RefreshObjectives`
  (if (`|EnumEquality` (`self.QuestState`) "NewEnumerator2")
    (for _array_element (`self.Objectives`)
      (if (not (`/Game/QuestSystem/Objectives/BP_Objective.IsCompleted` _array_element))
        (`/Game/QuestSystem/Objectives/BP_Objective.Evaluate` _array_element (`self.PlayerControllerRef`))))
    (`self.CheckQuestForCompleted`)))

(event `RefreshQuestState`
  (switch `/Game/QuestSystem/E_QuestStates` (`self.QuestState`)))

(fn `CheckQuestForAvailable`
  (locals (CurrentQuestPass :type Boolean))
  (if (`|EnumEquality` (`self.QuestState`) "NewEnumerator0")
    (if (>= (`KismetArrayLibrary.Array_Length` (`self.Conditions`)) 1)
      (switch `/Game/QuestSystem/E_QuestConditionGroupRule` (`self.ConditionGroupRule`)
        (:`NewEnumerator0`
          ; If All condition Needed
          ; Set true by default, then false if any of them is false
          ;
          ; If Any Condition Needed
          ; Set False by default, and then true if any of them is true
          (set `local.CurrentQuestPass` true))
        (:`NewEnumerator1`
          (set `local.CurrentQuestPass` false)))
      (for _array_element (`self.Conditions`)
        (bind _result (`/Game/QuestSystem/Conditions/BP_Condition.Evaluate` _array_element (`self.PlayerControllerRef`)))
        (if _result
          (switch `/Game/QuestSystem/E_QuestConditionGroupRule` (`self.ConditionGroupRule`)
            (:`NewEnumerator1`
              ; If Any Condition Needed
              ; Set False by default, and then true if any of them is true
              (set `local.CurrentQuestPass` true)
              (break)))
          (else
            (switch `/Game/QuestSystem/E_QuestConditionGroupRule` (`self.ConditionGroupRule`)
              (:`NewEnumerator0`
                ; If All condition Needed
                ; Set true by default, then false if any of them is false
                (set `local.CurrentQuestPass` false)
                (break))))))
      (if (`local.CurrentQuestPass`)
        (`self.SetQuestState` "NewEnumerator1"))
      (else
        ; No Conditions
        (`self.SetQuestState` "NewEnumerator1")))))

(fn `CheckQuestForCompleted`
  (locals (AllCompleted :type Boolean))
  (if (`|EnumEquality` (`self.QuestState`) "NewEnumerator2")
    (set `local.AllCompleted` true)
    (for _array_element (`self.Objectives`)
      (if (not (`/Game/QuestSystem/Objectives/BP_Objective.IsCompleted` _array_element))
        (set `local.AllCompleted` false)
        (break)))
    (if (`local.AllCompleted`)
      (`self.SetQuestState` "NewEnumerator3")
      (`/Game/Variant_Shooter/Blueprints/FirstPerson/BP_ShooterController.OnQuestStateChanged` (`self.PlayerControllerRef`) (`self.QuestID`) "NewEnumerator3"))))

(fn `OnObjectiveCompleted`
  (`self.RefreshObjectives`))

(fn `SetQuestState`
  (params (InNewState :type "/Game/QuestSystem/E_QuestStates Enum" :default "NewEnumerator0"))
  (bind _output_get (set `self.QuestState` InNewState))
  (switch `/Game/QuestSystem/E_QuestStates` _output_get
    (:`NewEnumerator1`
      (`self.RefreshObjectives`))
    (:`NewEnumerator2`
      (`self.RefreshObjectives`)
      (for _array_element (`self.Objectives`)
        (if (not (`/Game/QuestSystem/Objectives/BP_Objective.IsCompleted` _array_element))
          (add `/Game/QuestSystem/Objectives/BP_Objective.OnObjectiveCompleted` _array_element (`|CreateDelegate` :!event `OnObjectiveCompleted`)))))
    (:`NewEnumerator3`
      (for _array_element_2 (`self.Objectives`)
        (clear `/Game/QuestSystem/Objectives/BP_Objective.OnObjectiveCompleted` _array_element_2))
      (bind _ashud_shooter (cast `/Game/Variant_Shooter/UI/HUD_Shooter` (`PlayerController.GetHUD` (`self.PlayerControllerRef`))))
      (`/Game/UI/HUD/BP_QuestComplete_Notify.PlayBanner` (`/Game/Variant_Shooter/UI/HUD_Shooter.QuestCompleteBanner` _ashud_shooter) (`self.QuestName`)))))