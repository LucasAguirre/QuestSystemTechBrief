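; Quest objective that tracks how many times the player hits shooting targets and completes at a required count.
; Initialize stores the target ID, player character and required amount, and BindEvents and UnbindEvents manage a listener on the character's OnTargetHit event.
; OnShootTarget counts matching hits, treating a None or ANY ID as a wildcard, and signals completion once the count is met.
; Evaluate rechecks that count on demand.
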(event `Initialize`
  (params (TargetID :type Name) (PlayerCharacter :type "/Game/Variant_Shooter/Blueprints/FirstPerson/BP_FPShooter Object Reference") (RequiredAmount :type Integer))
  (set `self.Target ID` TargetID)
  (set `self.Player Character` PlayerCharacter)
  (set `self.RequiredImpactNumber` RequiredAmount))

(fn `BindEvents`
  (bind _player_character (`self.Player Character`))
  (`parent.BindEvents`)
  (`/Engine/EditorBlueprintResources/StandardMacros.IsValid` _player_character
    (:`Is Valid`
      (add `/Game/Variant_Shooter/Blueprints/FirstPerson/BP_FPShooter.OnTargetHit` _player_character (`|CreateDelegate` :!event `OnShootTarget`)))))

(fn `Evaluate`
  (params (Controller :type "/Game/Variant_Shooter/Blueprints/FirstPerson/BP_ShooterController Object Reference"))
  (returns (Result :type Boolean))
  (bind _returnvalue (<= (`self.RequiredImpactNumber`) (`self.ImpactNumber`)))
  (set `self.IsCompleted` _returnvalue)
  (return _returnvalue))

(fn `OnShootTarget`
  (params (InTargetId :type Name))
  (if (or (== (`local.InTargetId`) (`self.Target ID`)) (== (`self.Target ID`) "None") (== (`self.Target ID`) "ANY"))
    (`/Engine/EditorBlueprintResources/StandardMacros.IncrementInt` (`self.ImpactNumber`)
      (:`  `
        _)))
  (bind _output_get (set `self.IsCompleted` (<= (`self.RequiredImpactNumber`) (`self.ImpactNumber`))))
  (if _output_get
    (`self.OnObjectiveCompleted`)))

(fn `UnbindEvents`
  (bind _player_character (`self.Player Character`))
  (`parent.UnbindEvents`)
  (`/Engine/EditorBlueprintResources/StandardMacros.IsValid` _player_character
    (:`Is Valid`
      (remove `/Game/Variant_Shooter/Blueprints/FirstPerson/BP_FPShooter.OnTargetHit` _player_character (`|CreateDelegate` :!event `OnShootTarget`)))))