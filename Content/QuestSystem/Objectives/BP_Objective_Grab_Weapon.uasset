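; Quest objective that completes when the player owns a specific weapon class, or any weapon if no valid class is set.
; Initialization stores the class and character, then evaluates immediately, so an already owned weapon counts.
; Bind and unbind overrides hook the character's OnWeaponGrabbed event for pickup tracking.
; Evaluate checks the character's owned weapons until completion, then fires the objective-completed call.
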(event `Initialize`
  (params (WeaponClass :type "/Game/Variant_Shooter/Blueprints/Pickups/BP_WeaponBase Class Reference") (PlayerCharacter :type "/Game/Variant_Shooter/Blueprints/FirstPerson/BP_FPShooter Object Reference"))
  ; Unused for now, ideally each weapon type has an ID and we check for that if we want a  specific weapon
  (set `self.Weapon Class` WeaponClass)
  (set `self.Player Character` PlayerCharacter)
  (bind _result (`self.Evaluate` null))
  (if _result
    (set `self.IsCompleted` true)))

(event `OnPlayerPickUpWeapon`
  (params (WeaponClass :type "/Game/Variant_Shooter/Blueprints/Pickups/BP_WeaponBase Class Reference"))
  (`self.Evaluate` null))

(fn `BindEvents`
  (`parent.BindEvents`)
  (add `/Game/Variant_Shooter/Blueprints/FirstPerson/BP_FPShooter.OnWeaponGrabbed` (`self.Player Character`) (`|CreateDelegate` :!event `OnPlayerPickUpWeapon`)))

(fn `Evaluate`
  (params (Controller :type "/Game/Variant_Shooter/Blueprints/FirstPerson/BP_ShooterController Object Reference"))
  (returns (Result :type Boolean))
  (if (not (`self.IsCompleted`))
    (`|ExecutionSequence`
      (:`then_0`
        (if (`KismetSystemLibrary.IsValidClass` (`self.Weapon Class`))
          (bind _owned (`/Game/Variant_Shooter/Blueprints/FirstPerson/BP_FPShooter.Is Weapon Already Owned` (`self.Player Character`) (`self.Weapon Class`)))
          (set `self.IsCompleted` _owned)
          (else
            (set `self.IsCompleted` (`KismetArrayLibrary.Array_IsNotEmpty` (`/Game/Variant_Shooter/Blueprints/FirstPerson/BP_FPShooter.Owned Weapons` (`self.Player Character`)))))))
      (:`then_1`
        (if (`self.IsCompleted`)
          (`self.OnObjectiveCompleted`))
        (return (`self.IsCompleted`))))))

(fn `UnbindEvents`
  (`parent.UnbindEvents`)
  (remove `/Game/Variant_Shooter/Blueprints/FirstPerson/BP_FPShooter.OnWeaponGrabbed` (`self.Player Character`) (`|CreateDelegate` :!event `OnPlayerPickUpWeapon`)))