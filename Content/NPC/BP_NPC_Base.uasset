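; Base NPC that shows its name on a text element and handles player interaction with quest-aware dialogue.
; Interact queries the player controller's quest system by NPC ID and picks accept, repeat or completion text from the first quest's state.
; Without quests, it cycles through idle dialogue one line per interaction.
; ShowDialogue forwards lines to BP_ShooterController, passing the quest to advance for Available and Completed states.
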(event `self.ReceiveBeginPlay`
  (`TextRenderComponent.K2_SetText` (`self.NPCNameText`) (`self.NPC_Name`)))

(event `/Game/NPC/BPI_Interactable.Interact`
  (bind _asbp_shooter_controller (cast `/Game/Variant_Shooter/Blueprints/FirstPerson/BP_ShooterController` (`GameplayStatics.GetPlayerController` 0)))
  (bind _questlist (`/Game/QuestSystem/BP_QuestSystem.GetQuestsForNPC` (`/Game/Variant_Shooter/Blueprints/FirstPerson/BP_ShooterController.BP_QuestSystem` _asbp_shooter_controller) (`self.NPC_ID`)))
  (if (`KismetArrayLibrary.Array_IsEmpty` _questlist)
    (if (> (`KismetArrayLibrary.Array_Length` (`self.InteractDialogue`)) 0)
      (if (`KismetArrayLibrary.Array_IsValidIndex` (`self.InteractDialogue`) (`self.DialogueIndex`)) :!label _label
        (`self.ShowDialogue` (`|MakeArray` (`|GetArrayItem` (`self.InteractDialogue`) (`self.DialogueIndex`))))
        (`/Engine/EditorBlueprintResources/StandardMacros.IncrementInt` (`self.DialogueIndex`))
        (else
          (set `self.DialogueIndex` 0)
          (goto _label))))
    (else
      (bind _output (`|GetArrayItem` _questlist))
      (switch `/Game/QuestSystem/E_QuestStates` (`/Game/QuestSystem/BP_SimpleQuest.QuestState` _output)
        (:`NewEnumerator1`
          (`self.ShowDialogue` (`/Game/QuestSystem/BP_SimpleQuest.TextOnAccept` _output) _output))
        (:`NewEnumerator2`
          (`self.ShowDialogue` (`/Game/QuestSystem/BP_SimpleQuest.TextOnRepeat` _output)))
        (:`NewEnumerator3`
          (`self.ShowDialogue` (`/Game/QuestSystem/BP_SimpleQuest.TextOnComplete` _output) _output))))))

(fn `ShowDialogue`
  (params (InLines :type "Array of Text") (QuestToAdvance :type "/Game/QuestSystem/BP_SimpleQuest Object Reference"))
  (bind _asbp_shooter_controller (cast `/Game/Variant_Shooter/Blueprints/FirstPerson/BP_ShooterController` (`GameplayStatics.GetPlayerController` 0)))
  (`/Game/Variant_Shooter/Blueprints/FirstPerson/BP_ShooterController.NPCDialogue` _asbp_shooter_controller InLines QuestToAdvance))

(fn `UserConstructionScript`)